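; Target actor that awards the player a point when hit, then removes itself.
; The construction script caches the first MyPlayerController found through GetAllActorsOfClass as TargetReg.
; On Hit, it attaches a particle effect to the other component, plays a sound at world origin and increments PlayerPoints on that controller.
; It destroys itself after a short delay, with no guard against repeat hits during that window.
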(event EventBeginPlay)

(event Collision|EventHit
  (params (MyComp :type Primitive%20Component%20Object%20Reference) (Other :type Actor%20Object%20Reference) (OtherComp :type Primitive%20Component%20Object%20Reference) (bSelfMoved :type Boolean) (HitLocation :type Vector :default "0, 0, 0") (HitNormal :type Vector :default "0, 0, 0") (NormalImpulse :type Vector :default "0, 0, 0") (Hit :type Hit%20Result%20Structure%20%28by%20ref%29))
  ;[1 1 1] Target Hit
  (Effects|SpawnEmitterAttached "/Game/Effects/P_Hit.P_Hit" OtherComp "None")
  (Audio|PlaySoundatLocation "/Game/Sounds/Randomize_08.Randomize_08" "0, 0, 0" "0, 0, 0" 1.0 1.0 0.0 0 0 0)
  (Variables|/Game/Blueprints/MyPlayerController.MyPlayerController_C|SetPlayerPoints (Variables|Default|GetTargetReg) (+ (Variables|/Game/Blueprints/MyPlayerController.MyPlayerController_C|GetPlayerPoints (Variables|Default|GetTargetReg)) 1))
  (Utilities|FlowControl|Delay 0.2)
  (Actor|DestroyActor))

(event EventTick
  (params (DeltaSeconds :type Float%20%28single-precision%29)))

(fn ConstructionScript
  (bind _outactors (Actor|GetAllActorsOfClass "/Game/Blueprints/MyPlayerController.MyPlayerController_C"))
  (Variables|Default|SetTargetReg (Utilities|Array|Get(acopy) _outactors)))